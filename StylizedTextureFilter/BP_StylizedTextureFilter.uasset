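; Batch texture stylizer Blueprint that runs a Kuwahara material filter over an array of textures and exports the results to disk.
; CreateTexture loops the array, feeding each texture, its width and the Radius into a dynamic instance of MI_kuwahara.
; Each instance is drawn to a square RGBA8 render target sized by texture width, then exported as a .png-named file to a hardcoded D: folder.
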(event `CreateTexture`
  (`self.DrawMaterial2RenderTraget`))

(fn `DrawMaterial2RenderTraget`
  (for _array_element (`self.Texture`)
    (bind _returnvalue (`KismetMaterialLibrary.CreateDynamicMaterialInstance` "/Game/StylizedTextureFilter/MI_kuwahara.MI_kuwahara"))
    (bind _returnvalue_2 (`Texture2D.Blueprint_GetSizeX` _array_element))
    (`MaterialInstanceDynamic.SetScalarParameterValue` _returnvalue "TextureSize" (`KismetMathLibrary.Conv_IntToDouble` _returnvalue_2))
    (`MaterialInstanceDynamic.SetScalarParameterValue` _returnvalue "Radius" (`self.Radius`))
    (`MaterialInstanceDynamic.SetTextureParameterValue` _returnvalue "StalyeTexture" _array_element)
    (bind _returnvalue_3 (`KismetRenderingLibrary.CreateRenderTarget2D` _returnvalue_2 _returnvalue_2 "RTF_RGBA8"))
    (`KismetRenderingLibrary.DrawMaterialToRenderTarget` _returnvalue_3 _returnvalue)
    (`KismetRenderingLibrary.ExportRenderTarget` _returnvalue_3 "D:\\StylizedTextureFilte" (`KismetStringLibrary.Concat_StrStr` (`KismetSystemLibrary.GetDisplayName` _array_element) "StalyeTexture" ".png"))))

(fn `UserConstructionScript`)